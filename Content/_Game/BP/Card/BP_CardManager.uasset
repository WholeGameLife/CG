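; Card manager that offers three random cards in a selection screen, triggered by a debug key.
; DrawCards creates the card widget and picks three classes from the Card array, with repeats possible.
; ShowInUI constructs each as an object, calls ActiveCard, fills the widget's deck slots, then pauses the game with UI-only input.
; BeginPlay also loads CardDataTable into AllCards, which only disconnected older draw logic reads.
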(event EventBeginPlay
  (bind _carddatatable (Variables|Default|GetCardDataTable))
  (bind _outrownames (DataTable|GetDataTableRowNames _carddatatable))
  (for _array_element _outrownames
    (bind _returnvalue (Utilities|GetDataTableRow _carddatatable _array_element)
      (:then
        (Utilities|Array|Add (Variables|Default|GetAllCards) _returnvalue)))))

(event Collision|EventActorBeginOverlap
  (params (OtherActor :type Actor%20Object%20Reference)))

(event EventTick
  (params (DeltaSeconds :type Float%20%28single-precision%29)))

(event Input|KeyboardEvents|DebugKey0
  (params (Key :type Key%20Structure) (ActionValue :type Input%20Action%20Value%20Structure))
  (:Pressed
    (CallFunction|DrawCards)))

(fn ConstructionScript)

(fn DrawCards
  (bind _card (Variables|Default|GetCard))
  (bind _returnvalue (UserInterface|CreateWidget "/Game/UI/HUD/Card_UMG.Card_UMG_C"))
  (Variables|Default|SetCardUI _returnvalue)
  (Utilities|Array|Clear (Variables|Default|GetShowCards))
  (for _index (range 0 2)
    (Utilities|Array|Add (Variables|Default|GetShowCards) (Utilities|Array|Get(acopy) _card (Math|Random|RandomIntegerinRange 0 (- (Utilities|Array|Length _card) 1)))))
  (CallFunction|ShowinUI))

(fn ShowinUI
  (bind _returnvalue (Game|GetPlayerController 0))
  (bind _cardui (Variables|Default|GetCardUI))
  (bind _showcards (Variables|Default|GetShowCards))
  (bind _cardui_2 (Variables|Default|GetCardUI))
  (bind _returnvalue_2 (Game|ConstructObjectfromClass (Utilities|Array|Get(acopy) _showcards) 0))
  (Default|ActiveCard _returnvalue_2)
  (Variables|/Game/UI/HUD/Card_UMG.Card_UMG_C|SetFirstDeck _cardui_2 _returnvalue_2)
  (bind _returnvalue_3 (Game|ConstructObjectfromClass (Utilities|Array|Get(acopy) _showcards 1) 0))
  (Default|ActiveCard _returnvalue_3)
  (Variables|/Game/UI/HUD/Card_UMG.Card_UMG_C|SetSecondDeck _cardui_2 _returnvalue_3)
  (bind _returnvalue_4 (Game|ConstructObjectfromClass (Utilities|Array|Get(acopy) _showcards 2) 0))
  (Default|ActiveCard _returnvalue_4)
  (Variables|/Game/UI/HUD/Card_UMG.Card_UMG_C|SetThirdDeck _cardui_2 _returnvalue_4)
  (UserInterface|Viewport|AddtoViewport _cardui 0)
  (Game|SetGamePaused true)
  (bind _output_get (Variables|/Script/Engine.PlayerController|SetbShowMouseCursor _returnvalue true))
  (Input|SetInputModeUIOnly _returnvalue _cardui "DoNotLock" _output_get))