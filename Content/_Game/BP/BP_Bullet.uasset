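; BP_Bullet is a projectile actor that damages the player or a boss on hit, and self-destructs after a delay started from Tick.
; A sphere hit destroys it and switches on the hit actor's first tag.
; "Player" calls ApplyDamage on that BP_Player; any other tag calls it on the first actor found with that tag, if a BP_Boss.
; A disconnected tag-loop branch with per-enemy checks remains unused.
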(event OnComponentHit(Sphere)
  (params (HitComponent :type Primitive%20Component%20Object%20Reference) (OtherActor :type Actor%20Object%20Reference) (OtherComp :type Primitive%20Component%20Object%20Reference) (NormalImpulse :type Vector :default "0, 0, 0") (Hit :type Hit%20Result%20Structure%20%28by%20ref%29))
  (bind _tags (Variables|/Script/Engine.Actor|GetTags OtherActor))
  (bind _output (Utilities|Array|Get(acopy) _tags))
  (Actor|DestroyActor)
  (switch string (Utilities|String|ToString(Name) _output)
    (:Default
      (bind _outactors (Actor|GetAllActorswithTag _output))
      (bind _asbp_boss (Utilities|Casting|CastToBP_Boss (Utilities|Array|Get(acopy) _outactors)))
      (Default|ApplyDamage _asbp_boss))
    (:player
      (bind _asbp_player (Utilities|Casting|CastToBP_Player OtherActor))
      (Default|ApplyDamage _asbp_player))))

(event EventBeginPlay)

(event Collision|EventActorBeginOverlap
  (params (OtherActor :type Actor%20Object%20Reference)))

(event EventTick
  (params (DeltaSeconds :type Float%20%28single-precision%29))
  (Utilities|FlowControl|Delay 1e+01)
  (Actor|DestroyActor))

(fn ConstructionScript)