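; Boss enemy that chases the player and fires bullets at them until its health runs out.
; Each Tick while alive it moves toward player character 0, interpolates its rotation to face them and enables attacking; at zero health it destroys itself.
; PawnSensing sightings trigger a delayed attack that spawns BP_Bullet from two arrow components.
; ApplyDamage lowers Health, clamped between zero and MaxHealth.
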(event OnSeePawn(PawnSensing)
  (params (Pawn :type Pawn%20Object%20Reference))
  (if (Variables|Default|GetisAttackPlayer)
    (Utilities|FlowControl|Delay 1.0)
    (CallFunction|AttackPlayer)))

(event Custom|Follow%20Player
  (Pawn|Input|AddMovementInput (Math|Rotator|GetRotationXVector (Math|Rotator|FindLookatRotation (Transformation|GetActorLocation) (Transformation|GetActorLocation (Game|GetPlayerCharacter 0)))) 2.0 false)
  (Variables|Default|SetisAttackPlayer true)
  (Transformation|SetActorRotation (Math|Interpolation|RInterpTo (Transformation|GetActorRotation) (Math|Rotator|FindLookatRotation (Transformation|GetActorLocation) (Transformation|GetActorLocation (Game|GetPlayerCharacter 0))) 1.0 1e+01)))

(event Custom|Attack%20Player
  (bind _arrow1 (Variables|Default|GetArrow1))
  (bind _arrow (Variables|Default|GetArrow))
  (bind _returnvalue (Transformation|GetWorldTransform _arrow))
  (bind _returnvalue_2 (Transformation|GetWorldTransform _arrow1))
  (Game|SpawnActorfromClass "/Game/_Game/BP/BP_Bullet.BP_Bullet_C" (Math|Transform|MakeTransform (.location _returnvalue_2) (.rotation _returnvalue_2) "1.000000,1.000000,1.000000") "AlwaysSpawn" 0 0)
  (Game|SpawnActorfromClass "/Game/_Game/BP/BP_Bullet.BP_Bullet_C" (Math|Transform|MakeTransform (.location _returnvalue) (.rotation _returnvalue) "1.000000,1.000000,1.000000") "AlwaysSpawn" 0 0))

(event EventBeginPlay
  (Variables|Default|SetHealth (Variables|Default|GetMaxHealth)))

(event Collision|EventActorBeginOverlap
  (params (OtherActor :type Actor%20Object%20Reference)))

(event EventTick
  (params (DeltaSeconds :type Float%20%28single-precision%29))
  (if (> (Variables|Default|GetHealth) 0.0)
    (CallFunction|FollowPlayer)
    (else
      (Actor|DestroyActor))))

(fn ConstructionScript)

(fn ApplyDamage
  (if (not (<= (Variables|Default|GetHealth) 0.0))
    (Variables|Default|SetHealth (Math|Float|Clamp(Float) (- (Variables|Default|GetHealth) (Variables|Default|GetDamage)) 0.0 (Variables|Default|GetMaxHealth)))))