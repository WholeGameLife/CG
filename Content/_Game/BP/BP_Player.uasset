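; BP_Player is the player character, with health, twin-muzzle shooting, a pause menu and a death screen.
; BeginPlay creates the FPS and blood HUDs, and left click spawns bullets from two arrow components that ignore the player.
; Any overlap on its box subtracts clamped damage, and Tick polls health to swap the FPS HUD for the death HUD and destroy the actor.
; P opens the pause widget, pauses the game and switches to UI-only input.
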(event OnComponentBeginOverlap(Box)
  (params (OverlappedComponent :type Primitive%20Component%20Object%20Reference) (OtherActor :type Actor%20Object%20Reference) (OtherComp :type Primitive%20Component%20Object%20Reference) (OtherBodyIndex :type Integer) (bFromSweep :type Boolean) (SweepResult :type Hit%20Result%20Structure%20%28by%20ref%29))
  (CallFunction|ApplyDamage))

(event EventBeginPlay
  (bind _output_get (Variables|Default|SetMaxHealth 1e+02))
  (Variables|Default|SetHealth _output_get)
  (bind _returnvalue (UserInterface|CreateWidget "/Game/UI/HUD/FPSHUD.FPSHUD_C"))
  (bind _output_get_2 (Variables|Default|SetFPS _returnvalue))
  (bind _returnvalue_2 (UserInterface|CreateWidget "/Game/UI/BloodUI/BloodHUD.BloodHUD_C"))
  (bind _output_get_3 (Variables|Default|SetBlood _returnvalue_2))
  (UserInterface|Viewport|AddtoViewport _output_get_2 0)
  (bind _asbp_player (Utilities|Casting|CastToBP_Player (Game|GetPlayerCharacter 0)))
  (Variables|Default|Setplayer _asbp_player))

(event EventTick
  (params (DeltaSeconds :type Float%20%28single-precision%29))
  (bind _returnvalue (Game|GetPlayerController 0))
  (bind _fps (Variables|Default|GetFPS))
  (if (<= (Variables|Default|GetHealth) 0.0)
    (Utilities|IsValid _fps
      (:Is%20Valid
        (Widget|RemovefromParent _fps)
        (bind _returnvalue_2 (UserInterface|CreateWidget "/Game/UI/WinUI/DeadHUD.DeadHUD_C"))
        (bind _output_get (Variables|Default|SetDead _returnvalue_2))
        (UserInterface|Viewport|AddtoViewport _output_get 0)
        (bind _output_get_2 (Variables|/Script/Engine.PlayerController|SetbShowMouseCursor _returnvalue true))
        (Input|SetInputModeUIOnly _returnvalue _output_get "DoNotLock" _output_get_2)
        (Actor|DestroyActor)))))

(event Input|MouseEvents|LeftMouseButton
  (params (Key :type Key%20Structure :default "None"))
  (bind _arrow2 (Variables|Default|GetArrow2))
  (bind _returnvalue (Transformation|GetWorldTransform _arrow2))
  (:Pressed
    (bind _returnvalue_2 (Game|SpawnActorfromClass "/Game/_Game/BP/BP_Bullet.BP_Bullet_C" (Math|Transform|MakeTransform (.location _returnvalue) (.rotation _returnvalue) "1.000000,1.000000,1.000000") "AlwaysSpawn" 0 0))
    (Actor|SetOwner 0)
    (Collision|IgnoreActorwhenMoving (Variables|/Game/_Game/BP/BP_Bullet.BP_Bullet_C|GetSphere _returnvalue_2) (Variables|Default|Getplayer) true)))

(event Input|MouseEvents|LeftMouseButton
  (params (Key :type Key%20Structure :default "None"))
  (bind _arrow1 (Variables|Default|GetArrow1))
  (bind _returnvalue (Transformation|GetWorldTransform _arrow1))
  (:Pressed
    (bind _returnvalue_2 (Game|SpawnActorfromClass "/Game/_Game/BP/BP_Bullet.BP_Bullet_C" (Math|Transform|MakeTransform (.location _returnvalue) (.rotation _returnvalue) "1.000000,1.000000,1.000000") "AlwaysSpawn" 0 0))
    (Audio|PlaySound2D "/Engine/VREditor/Sounds/UI/Camera_Shutter.Camera_Shutter" 1.0 1.0 0.0 0 0)
    (Actor|SetOwner 0)
    (Collision|IgnoreActorwhenMoving (Variables|/Game/_Game/BP/BP_Bullet.BP_Bullet_C|GetSphere _returnvalue_2) (Variables|Default|Getplayer) true)))

(event Input|KeyboardEvents|P
  (params (Key :type Key%20Structure :default "None"))
  (bind _returnvalue (Game|GetPlayerController 0))
  (:Pressed
    (bind _returnvalue_2 (UserInterface|CreateWidget "/Game/UI/PauseUI/PauseHUD.PauseHUD_C"))
    (UserInterface|Viewport|AddtoViewport _returnvalue_2 0)
    (Variables|/Script/Engine.PlayerController|SetbShowMouseCursor _returnvalue true)
    (Game|SetGamePaused true)
    (Input|SetInputModeUIOnly _returnvalue _returnvalue_2 "DoNotLock" false)))

(fn ConstructionScript)

(fn ApplyDamage
  (if (not (<= (Variables|Default|GetHealth) 0.0))
    (bind _output_get (Variables|Default|SetHealth (Math|Float|Clamp(Float) (- (Variables|Default|GetHealth) (Variables|Default|GetDamage)) 0.0 (Variables|Default|GetMaxHealth))))
    (Development|PrintString (Utilities|String|ToString(Float) _output_get))))