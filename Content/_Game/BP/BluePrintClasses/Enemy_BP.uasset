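; Enemy pawn that chases the player and shoots when its PawnSensing component spots a pawn.
; Each sighting sets a seeing flag, starts an AI MoveTo toward player 0, and spawns a Bullet_BP above itself, launched by a forward velocity impulse.
; A timer starts on each sighting, but its event is empty and the flag is never cleared here.
; Any capsule overlap destroys the enemy.
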(event OnSeePawn(PawnSensing)
  (params (Pawn :type Pawn%20Object%20Reference))
  (Variables|Default|SetisSeeingplayer true)
  (CallFunction|FollowPlayer)
  (Utilities|Time|SetTimerbyEvent (delegate Custom|自定义事件) 3.0)
  (bind _returnvalue (Game|SpawnActorfromClass "/Game/_Game/BP/BluePrintClasses/Bullet_BP.Bullet_BP_C" (Math|Transform|MakeTransform (+ (Transformation|GetActorLocation) "0.000000,0.000000,100.000000") "0, 0, 0" "1.000000,1.000000,1.000000") "AlwaysSpawn" 0 0))
  (Physics|AddImpulse (Variables|/Script/Engine.StaticMeshActor|GetStaticMeshComponent _returnvalue) (* (Transformation|GetActorForwardVector) "1000.000000,1000.000000,0.000000") "None" true))

(event OnComponentBeginOverlap(CapsuleComponent)
  (params (OverlappedComponent :type Primitive%20Component%20Object%20Reference) (OtherActor :type Actor%20Object%20Reference) (OtherComp :type Primitive%20Component%20Object%20Reference) (OtherBodyIndex :type Integer) (bFromSweep :type Boolean) (SweepResult :type Hit%20Result%20Structure%20%28by%20ref%29))
  (Actor|DestroyActor))

(event Custom|FollowPlayer
  (if (Variables|Default|GetisSeeingplayer)
    (AI|AIMoveTo self "1.000000,1.000000,1.000000" (Game|GetPlayerCharacter 0) 5.0 false)))

(event Custom|自定义事件)

(fn ConstructionScript)