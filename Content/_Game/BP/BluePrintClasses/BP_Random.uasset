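; BP_Random is a spawner that repeatedly places waves of BP_Boss actors at random world positions.
; BeginPlay fires a custom event that re-arms a non-looping 13-second timer on itself, then spawns bosses in a loop driven by the 生成数量 (spawn count) variable.
; Each position is randomized twice, as a random point in a box whose center is itself random around the world origin, independent of the spawner's location.
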(event Custom|自定义事件
  (Utilities|Time|SetTimerbyEvent (delegate Custom|自定义事件) 13.0)
  (for _index (range 0 (Variables|Default|Get生成数量))
    (Game|SpawnActorfromClass "/Game/_Game/BP/BP_Boss.BP_Boss_C" (Math|Transform|MakeTransform (Math|Random|RandomPointinBoundingBox (Math|Vector|MakeVector (Math|Random|RandomFloatinRange -1.5e+03 1.5e+03) (Math|Random|RandomFloatinRange -8e+02 8e+02) (Math|Random|RandomFloatinRange -8e+02 8e+02)) "1500.000000,800.000000,800.000000") "0, 0, 0" "1.000000,1.000000,1.000000") "Undefined" 0 0)))

(event EventBeginPlay
  (CallFunction|自定义事件))

(fn ConstructionScript)